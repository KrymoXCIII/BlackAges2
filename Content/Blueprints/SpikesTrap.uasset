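; Spikes trap actor that damages zombie and boss characters when they begin overlapping it.
; On overlap, a Sequence tries casts to ZombieCharacter and BossCharacter, subtracting TrapDamage directly from the matching health variable instead of using ApplyDamage.
; Damage lands once per overlap start, with no clamping, death check or effect on other actor types in this graph.
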(event `self.ReceiveActorBeginOverlap`
  (params (OtherActor :type "Actor Object Reference"))
  (`|ExecutionSequence`
    (:`then_0`
      (bind _aszombie_character (cast `/Game/Blueprints/CHARACTERS/ZombieCharacter` OtherActor))
      (set `/Game/Blueprints/CHARACTERS/ZombieCharacter.ZOMBIEHEALTH` (- (`/Game/Blueprints/CHARACTERS/ZombieCharacter.ZOMBIEHEALTH` _aszombie_character) (`self.TrapDamage`)) _aszombie_character))
    (:`then_1`
      (bind _asboss_character (cast `/Game/Blueprints/CHARACTERS/BossCharacter` OtherActor))
      (set `/Game/Blueprints/CHARACTERS/BossCharacter.BOSSHEALTH` (- (`/Game/Blueprints/CHARACTERS/BossCharacter.BOSSHEALTH` _asboss_character) (`self.TrapDamage`)) _asboss_character))))

(fn `UserConstructionScript`)