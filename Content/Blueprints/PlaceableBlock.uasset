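; PlaceableBlock is a block that starts as a non-colliding preview and becomes solid when placed.
; On BeginPlay it saves the mesh's first material, swaps in a preview material and disables collision.
; The Placed event restores the saved material and turns on query and physics collision.
; Nothing in the Blueprint calls Placed or moves the block.
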(event `self.ReceiveBeginPlay`
  (bind _staticmesh (`self.StaticMesh`))
  (set `self.DefaultMaterial` (`PrimitiveComponent.GetMaterial` _staticmesh 0))
  (`PrimitiveComponent.SetMaterial` _staticmesh 0 "/Game/Materials/PreviewMat.PreviewMat")
  (`PrimitiveComponent.SetCollisionEnabled` (`self.StaticMesh`) "NoCollision"))

(event `Placed`
  (`PrimitiveComponent.SetMaterial` (`self.StaticMesh`) 0 (`self.DefaultMaterial`))
  (`PrimitiveComponent.SetCollisionEnabled` (`self.StaticMesh`) "QueryAndPhysics"))

(fn `UserConstructionScript`)