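; BP_Shop is a shop actor that switches the player into a shop view when they walk into its ShopTrigger.
; On overlap by player 0's character, it blends the view target to itself, sets UI-only input with a visible cursor and disables character input.
; It also explicitly leaves the character unhidden.
; The graph creates no shop widget and has no logic to exit or restore control.
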(event `self.ShopTrigger.OnComponentBeginOverlap`
  (params (OverlappedComponent :type "PrimitiveComponent Object Reference") (OtherActor :type "Actor Object Reference") (OtherComp :type "PrimitiveComponent Object Reference") (OtherBodyIndex :type Integer) (bFromSweep :type Boolean) (SweepResult :type "HitResult Structure (by ref)"))
  (bind _returnvalue (`GameplayStatics.GetPlayerController` 0))
  (bind _returnvalue_2 (`GameplayStatics.GetPlayerCharacter` 0))
  (if (== OtherActor (`GameplayStatics.GetPlayerCharacter` 0))
    (`PlayerController.SetViewTargetWithBlend` (`GameplayStatics.GetPlayerController` 0) self 2.0 "VTBlend_Linear" 0.0 false)
    (`WidgetBlueprintLibrary.SetInputMode_UIOnlyEx` _returnvalue null)
    (set `PlayerController.bShowMouseCursor` true _returnvalue)
    (`self.SetActorHiddenInGame` _returnvalue_2 false)
    (`self.DisableInput` _returnvalue_2 (`GameplayStatics.GetPlayerController` 0))))

(fn `UserConstructionScript`)