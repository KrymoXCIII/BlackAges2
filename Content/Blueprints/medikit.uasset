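; Medikit pickup actor that restores 20 health and then destroys itself.
; On any overlap it casts player 0's character to PlayerCharacter and adds to PLAYERHEALTH unless it equals exactly 100, without checking which actor overlapped.
; A separate Interact event heals the passed Character's LifeActually when its truncated value is below 100, dropping fractions.
; Neither path clamps the result to 100.
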(event `self.ReceiveActorBeginOverlap`
  (params (OtherActor :type "Actor Object Reference"))
  (bind _asdefault_character (cast `/Game/Blueprints/CHARACTERS/PlayerCharacter` (`GameplayStatics.GetPlayerCharacter` 0)))
  (bind _playerhealth (`/Game/Blueprints/CHARACTERS/PlayerCharacter.PLAYERHEALTH` _asdefault_character))
  (if (!= _playerhealth 100.0)
    (set `/Game/Blueprints/CHARACTERS/PlayerCharacter.PLAYERHEALTH` (+ _playerhealth 20.0) _asdefault_character)
    (`self.K2_DestroyActor` self)))

(event `/Game/Blueprints/Interfaces/I_Interaction.Interact`
  (params (Character :type "/Game/Blueprints/CHARACTERS/PlayerCharacter Object Reference"))
  (bind _life_actually (`/Game/Blueprints/CHARACTERS/PlayerCharacter.Life_Actually` Character))
  (if (< (`KismetMathLibrary.FTrunc` _life_actually) 100)
    (set `/Game/Blueprints/CHARACTERS/PlayerCharacter.Life_Actually` (`KismetMathLibrary.Conv_IntToDouble` (+ (`KismetMathLibrary.FTrunc` _life_actually) 20)) Character)
    (`self.K2_DestroyActor`)))

(fn `UserConstructionScript`)