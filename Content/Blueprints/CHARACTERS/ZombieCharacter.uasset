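; Enemy zombie character that attacks the player in melee and awards random EXP when killed.
; AttackPlayer plays a montage and times a strike window, during which Tick damages the player if the right hand overlaps them, throttled by a Hit flag.
; Tick also polls health, triggering ragdoll death, AI unpossession and delayed destruction.
; The sword and axe damage-taking logic here is disconnected, so nothing in this Blueprint lowers zombie health.
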(event `self.ReceiveActorBeginOverlap`
  (params (OtherActor :type "Actor Object Reference")))

(event `self.ReceiveBeginPlay`
  (bind _output_get (set `self.ZOMBIEHEALTH` 100.0))
  (bind _aswbp_enemy_health_bar (cast `/Game/UI/WBP_EnemyHealthBar` (`WidgetComponent.GetWidget` (`self.HealthBar`))))
  (set `/Game/UI/WBP_EnemyHealthBar.HealthDisplay` _output_get _aswbp_enemy_health_bar))

(event `Attack Player`
  (`|ExecutionSequence`
    (:`then_0`
      (`|PlayMontage` (`self.Mesh`) "/Game/ANIMS/ZOMBIE/RETARGETED/zombie_attack_MontageATTACK.zombie_attack_MontageATTACK"
        (:`then`
          (cast `/Game/Blueprints/CHARACTERS/PlayerCharacter` (`GameplayStatics.GetPlayerCharacter` 0))
          (`KismetSystemLibrary.Delay` 1.2)
          (set `self.isStriking` false))))
    (:`then_1`
      (`KismetSystemLibrary.Delay` 0.5)
      (set `self.isStriking` true))))

(event `self.ReceiveTick`
  (params (DeltaSeconds :type "Float (single-precision)"))
  ;[1 0.9903 0.07997] EVENT TICK
  (`|ExecutionSequence`
    (:`then_0`
      ;;[1 0 0.01768] CHECK IF DEAD
      (if (`self.isDead`)
        _
        (elif (<= (`self.ZOMBIEHEALTH`) 0.0)
          (`KismetSystemLibrary.PrintString` "ZOMBIE IS DEAD")
          (`GameplayStatics.PlaySound2D` "/Game/EasyBuildingSystem/Audio/Sounds/UI/SFX_UI_Click_002.SFX_UI_Click_002" 1.0 1.0 0.0 null null)
          (bind _asplayer_character (cast `/Game/Blueprints/CHARACTERS/PlayerCharacter` (`GameplayStatics.GetPlayerCharacter` 0)))
          (`/Game/Blueprints/CHARACTERS/PlayerCharacter.Add EXP` _asplayer_character (`KismetMathLibrary.RandomIntegerInRange` 4 7))
          (`self.EnterDeadState`)
          (`KismetSystemLibrary.Delay` 10.0)
          (`self.K2_DestroyActor`))))
    (:`then_1`
      (if (`self.isStriking`)
        (if (`self.Player Colliding`)
          (bind _asplayer_character_2 (cast `/Game/Blueprints/CHARACTERS/PlayerCharacter` (stale `self.RightHand.OnComponentBeginOverlap` OtherActor)))
          (if (not (`self.Hit`))
            (set `self.Hit` true)
            (`KismetSystemLibrary.PrintString` "HIT" true true (struct :`R` 0.18964 :`G` 1.0 :`A` 1.0))
            (`GameplayStatics.PlaySound2D` "/Game/EasyBuildingSystem/Audio/Sounds/Interactions/Mining/SC_Pickaxe_Hit.SC_Pickaxe_Hit" 1.0 1.0 0.0 null null)
            (`/Game/Blueprints/CHARACTERS/PlayerCharacter.DamageIndicator` _asplayer_character_2 true)
            (set `/Game/Blueprints/CHARACTERS/PlayerCharacter.PLAYERHEALTH` (`KismetMathLibrary.FClamp` (- (`/Game/Blueprints/CHARACTERS/PlayerCharacter.PLAYERHEALTH` _asplayer_character_2) 15.0) 0.0 100.0) _asplayer_character_2)
            (`self.PlayAnimMontage` _asplayer_character_2 "/Game/ANIMS/ZOMBIE/RETARGETED/PLAYER_impact_Montage.PLAYER_impact_Montage" 1.0 "None")
            (`GameplayStatics.PlaySound2D` "/Game/EasyBuildingSystem/Audio/Sounds/Interactions/Chopping/SC_Hatchet_Hit.SC_Hatchet_Hit" 1.0 1.0 0.0 null null)
            (`KismetSystemLibrary.Delay` 0.5)
            (set `self.Hit` false)
            (`KismetSystemLibrary.Delay` 0.2)
            (`/Game/Blueprints/CHARACTERS/PlayerCharacter.DamageIndicator` _asplayer_character_2 false)))))))

(event `self.RightHand.OnComponentBeginOverlap`
  (params (OverlappedComponent :type "PrimitiveComponent Object Reference") (OtherActor :type "Actor Object Reference") (OtherComp :type "PrimitiveComponent Object Reference") (OtherBodyIndex :type Integer) (bFromSweep :type Boolean) (SweepResult :type "HitResult Structure (by ref)"))
  ;[1 0.9903 0.07997] EVENT TICK
  (cast `/Game/Blueprints/CHARACTERS/PlayerCharacter` OtherActor)
  (set `self.Player Colliding` true))

(event `self.RightHand.OnComponentEndOverlap`
  (params (OverlappedComponent :type "PrimitiveComponent Object Reference") (OtherActor :type "Actor Object Reference") (OtherComp :type "PrimitiveComponent Object Reference") (OtherBodyIndex :type Integer))
  ;[1 0.9903 0.07997] EVENT TICK
  (cast `/Game/Blueprints/CHARACTERS/PlayerCharacter` OtherActor)
  (set `self.Player Colliding` false))

(fn `decrease life`
  (if (<= (`KismetMathLibrary.FClamp` (- 0.0 1.0)) 0.0)
    _))

(fn `Def Base stat Actually`)

(fn `Def init stat perso`)

(fn `EnterDeadState`
  (set `self.isDead` true)
  (`ActorComponent.K2_DestroyComponent` (`self.HealthBar`))
  (`ActorComponent.K2_DestroyComponent` (`self.CapsuleComponent`))
  (`Controller.UnPossess` (`AIBlueprintHelperLibrary.GetAIController` self))
  (`self.DetachFromControllerPendingDestroy` self)
  (`self.EnterRagdollState`))

(fn `EnterRagdollState`
  (`PrimitiveComponent.SetSimulatePhysics` (`self.Mesh`) true))

(fn `NewFunction_0`)

(fn `UserConstructionScript`)