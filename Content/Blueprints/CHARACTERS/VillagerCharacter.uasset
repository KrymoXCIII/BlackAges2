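; VillagerCharacter is an AI-driven villager that cycles endlessly between work, eat and sleep locations.
; On BeginPlay it uses AIMoveTo to walk to WorkPos.
; Overlapping WorkPos, EatPos or SleepPos starts a fixed delay, then a move to the next stop in that work-eat-sleep order.
; A GoTo function that sets the actor's location with sweep is defined but not called here.
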(event `self.ReceiveBeginPlay`
  (`|AIMoveTo` self (`self.K2_GetActorLocation` (`self.WorkPos`)) null))

(event `self.ReceiveActorBeginOverlap`
  (params (OtherActor :type "Actor Object Reference"))
  (bind _workpos (`self.WorkPos`))
  (bind _sleeppos (`self.SleepPos`))
  (bind _eatpos (`self.EatPos`))
  (if (== OtherActor _sleeppos)
    (`KismetSystemLibrary.Delay` 5.0)
    (`|AIMoveTo` self (`self.K2_GetActorLocation` _workpos) null)
    (elif (== OtherActor _workpos)
      (`KismetSystemLibrary.Delay` 5.0)
      (`|AIMoveTo` self (`self.K2_GetActorLocation` _eatpos) null)
      (elif (== _eatpos OtherActor)
        (`KismetSystemLibrary.Delay` 5.0)
        (`|AIMoveTo` self (`self.K2_GetActorLocation` _sleeppos) null)))))

(fn `GoTo`
  (params (Location :type "Vector Structure"))
  (`self.K2_SetActorLocation` self Location true false))

(fn `UserConstructionScript`)