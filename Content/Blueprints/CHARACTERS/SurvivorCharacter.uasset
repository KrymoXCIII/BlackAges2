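; SurvivorCharacter is a survivor character that follows the first player's character while its FollowPlayerActive flag is on.
; Tick stores the player reference and calls FollowPlayer every frame, which also re-calls itself after a short delay.
; FollowPlayer uses AIMoveTo toward the player's current location when at or beyond a set distance, and targets the survivor itself when closer, effectively holding position.
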(event `self.ReceiveTick`
  (params (DeltaSeconds :type "Float (single-precision)"))
  (bind _asplayer_character (cast `/Game/Blueprints/CHARACTERS/PlayerCharacter` (`GameplayStatics.GetPlayerCharacter` 0)))
  (set `self.CharacterRef` _asplayer_character)
  (`self.FollowPlayer`))

(event `self.ReceiveBeginPlay`)

(event `FollowPlayer`
  (if (`self.followPlayerActive`)
    (if (>= (`self.GetDistanceTo` (`self.CharacterRef`)) 300.0)
      (`|AIMoveTo` self (`self.K2_GetActorLocation` (`self.CharacterRef`)) null
        (:`then`
          _))
      (else
        (`|AIMoveTo` self (0.0 0.0 0.0) self
          (:`then`
            _))))
    (`KismetSystemLibrary.Delay` 0.2)
    (`self.FollowPlayer`)))

(fn `UserConstructionScript`)