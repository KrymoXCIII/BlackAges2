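; Player character Blueprint handling movement, FPS/TPS camera switching, pause menu, item pickup and melee combat.
; Tagged overlapping items attach to a hand socket and drop via downward trace; held items enable FlipFlop-alternated attack montages.
; BeginPlay sets up health, UI and a looping timer; functions cover death with ragdoll and AI-perception removal, EXP levelling and damage overlay.
; Zombie damage, smooth capsule crouch and weapon-hitbox logic are disconnected.
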(event `InputAction|PAUSE GAME` :paused true
  (params (Key :type "Key Structure"))
  (bind _returnvalue (`GameplayStatics.GetPlayerController` 0))
  (bind _pause_menu_ref (`self.Pause Menu REF`))
  ;[1 1 1] Pause
  (:`Pressed`
    (`/Engine/EditorBlueprintResources/StandardMacros.IsValid` null
      (:`Is Valid`
        _)
      (:`Is Not Valid`
        (bind _returnvalue_2 (`|CreateWidget` "/Game/Imported/UI/Import/PausedMenuWidget.PausedMenuWidget_C"))
        (set `self.Pause Menu REF` _returnvalue_2)))
    (if (`GameplayStatics.IsGamePaused`)
      (`Widget.RemoveFromParent` _pause_menu_ref)
      (`GameplayStatics.SetGamePaused` false)
      (set `PlayerController.bShowMouseCursor` false _returnvalue)
      (`WidgetBlueprintLibrary.SetInputMode_GameOnly` _returnvalue)
      (else
        (`UserWidget.AddToViewport` _pause_menu_ref 0)
        (`GameplayStatics.SetGamePaused` true)
        (set `PlayerController.bShowMouseCursor` true _returnvalue)
        (`WidgetBlueprintLibrary.SetInputMode_GameAndUIEx` _returnvalue _pause_menu_ref "LockInFullscreen" false)))))

(event `CheckHitt`)

(event `self.ReceiveActorBeginOverlap`
  (params (OtherActor :type "Actor Object Reference"))
  ;[0.219 1 0] BEGIN OVERLAP
  (`|ExecutionSequence`
    (:`then_1`
      (message `/Game/Blueprints/Interfaces/I_Interaction.Interact` OtherActor self))))

(event `self.ReceiveTick`
  (params (DeltaSeconds :type "Float (single-precision)"))
  ;[1 0.8557 0] EVENT TICK
  (`|ExecutionSequence`))

(event `self.ReceiveBeginPlay`
  (bind _returnvalue (`GameplayStatics.GetPlayerController` 0))
  ;[0 0.007759 1] BEGINPLAY
  (`|ExecutionSequence`
    (:`then_0`
      (set `self.CapsuleHalfHeight` (`CapsuleComponent.CapsuleHalfHeight` (`self.CapsuleComponent`))))
    (:`then_1`
      (set `self.PLAYERHEALTH` 100.0))
    (:`then_2`
      (`self.Def init stat perso`))
    (:`then_3`
      (`KismetSystemLibrary.K2_SetTimer` self (`self.decrement_life_name`) 5.0 true))
    (:`then_4`
      (bind _returnvalue_2 (`|CreateWidget` "/Game/Imported/UI/UserInterface.UserInterface_C" _returnvalue))
      (`UserWidget.AddToViewport` _returnvalue_2 0)
      (`WidgetBlueprintLibrary.SetInputMode_GameOnly` _returnvalue))
    (:`then_5`
      (`self.Def Base stat Actually`))
    (:`then_6`
      (bind _returnvalue_3 (`|CreateWidget` "/Game/UI/WBP_DamageRedScreen.WBP_DamageRedScreen_C"))
      (set `self.DamageWidgetREF` _returnvalue_3))))

(event `InputAction|PICKUP/INTERACT`
  (params (Key :type "Key Structure"))
  ;[0.3385 0.08093 0.07756] PICKUP/INTERACT
  (:`Pressed`
    (if (not (`self.isHolding`))
      (for _array_element (`self.GetOverlappingActors` "/Script/Engine.Actor")
        (if (`self.ActorHasTag` _array_element "PICKUPABLE")
          ;;[0.2251 1 0.1025] PICKUP
          (bind _output_get (set `self.HELD_ITEM` _array_element))
          (`self.K2_AttachToComponent` _output_get (`self.Mesh`) "AxeHandSocket" "SnapToTarget" "SnapToTarget" "SnapToTarget" true)
          (set `self.isHolding` true)
          (break))))))

(event `InputAction|WALK`
  (params (Key :type "Key Structure"))
  (bind _charactermovement (`self.CharacterMovement`))
  ;[0 0.3762 0.6458] DEPLACEMENTS
  (:`Pressed`
    (set `CharacterMovementComponent.MaxWalkSpeed` 300.0 _charactermovement))
  (:`Released`
    (set `CharacterMovementComponent.MaxWalkSpeed` 500.0 _charactermovement)))

(event `InputAction|SPRINT`
  (params (Key :type "Key Structure"))
  (bind _charactermovement (`self.CharacterMovement`))
  ;[0 0.3762 0.6458] DEPLACEMENTS
  (:`Pressed`
    (set `CharacterMovementComponent.MaxWalkSpeed` 1000.0 _charactermovement))
  (:`Released`
    (set `CharacterMovementComponent.MaxWalkSpeed` 500.0 _charactermovement)))

(event `InputAxis|FW/BW`
  (params (AxisValue :type "Float (single-precision)"))
  ;[0 0.3762 0.6458] DEPLACEMENTS
  (if (< AxisValue 0.0)
    (set `self.bUseControllerRotationYaw` true)
    (else
      (set `self.bUseControllerRotationYaw` false)))
  (`self.AddMovementInput` (`KismetMathLibrary.GetForwardVector` (`KismetMathLibrary.MakeRotator` 0.0 0.0 (.yaw (`self.GetControlRotation`)))) AxisValue))

(event `Key|LeftMouseButton`
  (params (Key :type "Key Structure"))
  (bind _mesh (`self.Mesh`))
  ;[1 0 0] ATTACK
  (:`Pressed`
    (if (`self.isHolding`)
      (if (not (`self.isStriking`))
        (`|ExecutionSequence`
          (:`then_0`
            (`/Engine/EditorBlueprintResources/StandardMacros.FlipFlop`
              (:`A`
                (set `self.isStriking` true)
                (`KismetSystemLibrary.PrintString` "ON")
                (`|PlayMontage` _mesh "/Game/ANIMS/ZOMBIE/RETARGETED/PLAYER_attack_MontageATTACK1.PLAYER_attack_MontageATTACK1"
                  (:`then`
                    (`KismetSystemLibrary.Delay` 0.8))))
              (:`B`
                (set `self.isStriking` true)
                (`KismetSystemLibrary.PrintString` "ON")
                (`|PlayMontage` _mesh "/Game/ANIMS/ZOMBIE/RETARGETED/PLAYER_attack_MontageATTACK2.PLAYER_attack_MontageATTACK2" 1.5
                  (:`then`
                    (`KismetSystemLibrary.Delay` 0.8)))))
            (`KismetSystemLibrary.PrintString` "OFF")
            (set `self.isStriking` false))
          (:`then_1`
            ;[0.5781 0.01093 0] BLOCK CAMERA DURING ATTACK
            (bind _asplayer_character (cast `/Game/Blueprints/CHARACTERS/PlayerCharacter` (`GameplayStatics.GetPlayerCharacter` 0)))
            (set `Pawn.bUseControllerRotationYaw` true _asplayer_character)
            (`KismetSystemLibrary.Delay` 1.5)
            (if (not (`self.isFPS`))
              (set `Pawn.bUseControllerRotationYaw` false _asplayer_character))))))))

(event `InputAxis|RIGHT/LEFT`
  (params (AxisValue :type "Float (single-precision)"))
  ;[0 0.3762 0.6458] DEPLACEMENTS
  (`self.AddMovementInput` (`KismetMathLibrary.GetRightVector` (`KismetMathLibrary.MakeRotator` 0.0 0.0 (.yaw (`self.GetControlRotation`)))) AxisValue))

(event `InputAction|DROP`
  (params (Key :type "Key Structure"))
  (bind _held_item (`self.HELD_ITEM`))
  ;[0.3032 1 0.1758] DROP
  (:`Pressed`
    (if (`self.isHolding`)
      (`|ExecutionSequence`
        (:`then_0`
          (bind (_outhit _returnvalue) (`KismetSystemLibrary.LineTraceSingle` (`self.K2_GetActorLocation`) (- (`self.K2_GetActorLocation`) (0.0 0.0 500.0)) "TraceTypeQuery1"))
          (if _returnvalue
            (`self.K2_DetachFromActor` _held_item "KeepWorld" "KeepWorld" "KeepWorld")
            (`self.K2_SetActorTransform` _held_item (`KismetMathLibrary.MakeTransform` (+ (`.Location` (`GameplayStatics.BreakHitResult` _outhit)) (0.0 0.0 3.0)) (struct :`Roll` -90.0)) false false)
            (set `self.isHolding` false)))))))

(event `InputAxis|LOOK UP/DOWN`
  (params (AxisValue :type "Float (single-precision)"))
  ;[0.1117 1 0.4183] ROTATIONS
  (`self.AddControllerPitchInput` (`KismetMathLibrary.FClamp` AxisValue -5.0 5.0)))

(event `InputAxis|LOOK RIGHT/LEFT`
  (params (AxisValue :type "Float (single-precision)"))
  ;[0.1117 1 0.4183] ROTATIONS
  (`self.AddControllerYawInput` (`KismetMathLibrary.FClamp` AxisValue -5.0 5.0)))

(event `InputAction|CAMERA SWITCH`
  (params (Key :type "Key Structure"))
  (bind _fpscamera (`self.FPSCamera`))
  (bind _tpscamera (`self.TPSCamera`))
  ;[0.1264 0.1388 1] CAMERA SWITCH
  (:`Pressed`
    (`/Engine/EditorBlueprintResources/StandardMacros.FlipFlop`
      (:`A`
        (`ActorComponent.SetActive` _fpscamera true false)
        (`ActorComponent.SetActive` _tpscamera false false)
        (set `self.isFPS` true)
        (set `self.bUseControllerRotationYaw` true))
      (:`B`
        (`ActorComponent.SetActive` _tpscamera true false)
        (`ActorComponent.SetActive` _fpscamera false false)
        (set `self.isFPS` false)
        (set `self.bUseControllerRotationYaw` false)))))

(event `InputAction|JUMP`
  (params (Key :type "Key Structure"))
  ;[0.3121 0.3351 1] SAUT ET S'ACCROUPIR
  (:`Pressed`
    (`self.PlayAnimMontage` "/Game/ANIMS/CHARACTER/PlayerJumpMontage.PlayerJumpMontage")
    (`self.Jump`)))

(event `InputAction|CROUCH`
  (params (Key :type "Key Structure"))
  ;[0.3121 0.3351 1] SAUT ET S'ACCROUPIR
  (:`Pressed`
    (`self.StartCrouch`))
  (:`Released`
    (`self.StopCrouch`)))

(event `StartCrouch`
  ;[0.2113 0.2598 1] SMOOTH CROUCH
  (set `self.IsCrouched` true)
  (set `CharacterMovementComponent.MaxWalkSpeed` 250.0 (`self.CharacterMovement`)))

(event `StopCrouch`
  ;[0.2113 0.2598 1] SMOOTH CROUCH
  (set `self.IsCrouched` false)
  (set `CharacterMovementComponent.MaxWalkSpeed` 500.0 (`self.CharacterMovement`)))

(fn `Add EXP`
  (params (EXP :type Integer))
  (returns (Level :type Integer))
  (bind _output_get (set `self.EXP` (+ EXP (`self.EXP`))))
  (if (>= _output_get (`self.EXP Needed`))
    (`/Engine/EditorBlueprintResources/StandardMacros.IncrementInt` (`self.Level`)
      (:`  `
        (set `self.EXP` (- (`self.EXP`) (`self.EXP Needed`)))
        (set `self.EXP Needed` (`KismetMathLibrary.Clamp` (`KismetMathLibrary.FTrunc` (* (`self.EXP Needed`) 1.2)) 0 1000))
        (`GameplayStatics.PlaySound2D` "/Game/Sounds/LevelUp.LevelUp" 1.0 1.0 0.0 null null)
        (return (`self.Level`))))))

(fn `CheckHit`)

(fn `DamageIndicator`
  (params (AddToScreen :type Boolean))
  (bind _damagewidgetref (`self.DamageWidgetREF`))
  (if AddToScreen
    (`UserWidget.AddToViewport` _damagewidgetref 0)
    (else
      (`/Game/UI/WBP_DamageRedScreen.FadeOut` _damagewidgetref))))

(fn `Def Base stat Actually`
  (set `self.PLAYERHEALTH` (`self.Life_base`)))

(fn `Def init stat perso`
  (set `self.Life_base` 100.0))

(fn `EnterDeathState`
  (bind _returnvalue (`GameplayStatics.GetPlayerController` 0))
  (bind _returnvalue_2 (`|CreateWidget` "/Game/UI/WBP_DeathScreen.WBP_DeathScreen_C" _returnvalue))
  (`UserWidget.AddToViewport` _returnvalue_2 0)
  (`self.DisableInput` self _returnvalue)
  (set `self.isDead` true)
  (`self.EnterRagdollState`)
  (`AIPerceptionStimuliSourceComponent.UnregisterFromSense` (`self.AIPerceptionStimuliSource`) "/Script/AIModule.AISense_Sight")
  (`AIPerceptionStimuliSourceComponent.UnregisterFromPerceptionSystem` (`self.AIPerceptionStimuliSource`)))

(fn `EnterRagdollState`
  (`PrimitiveComponent.SetSimulatePhysics` (`self.Mesh`) true))

(fn `UserConstructionScript`)