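; BP_Shotgun is a gun Blueprint that fires bursts of randomly spread projectiles from its spawn point.
; Fire_Start shoots immediately and runs a looping timer, paced by fire rate and the player's attack speed, until Fire_Stop clears it.
; Each projectile costs one ammo and takes damage scaled by player attack multipliers.
; Firing on empty triggers a delayed refill from reserve ammo, alongside a separate Reload event.
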(event `Reload`
  (bind _ammomax (`self.AmmoMax`))
  (set `self.AmmoTotal` (- (`self.AmmoTotal`) (- _ammomax (`self.Ammo`))))
  (set `self.Ammo` _ammomax))

(event `Fire_Stop`
  (`KismetSystemLibrary.K2_ClearAndInvalidateTimerHandle` (stale `Fire_Start` _returnvalue_2)))

(event `Fire_Start`
  (if (not (`self.timerRunning`))
    (bind _asplayer_character (cast `/Game/Blueprints/CHARACTERS/PlayerCharacter` (`GameplayStatics.GetPlayerCharacter` 0)))
    (`self.Fire_Projectile`)
    (set `self.timerRunning` true)
    (bind _returnvalue (/ 1.0 (* (`self.FireRate`) (`/Game/Blueprints/CHARACTERS/PlayerCharacter.Att_speed_gun Mul` _asplayer_character))))
    (bind _returnvalue_2 (`KismetSystemLibrary.K2_SetTimerDelegate` (delegate `Fire_Projectile`) _returnvalue true))
    (`KismetSystemLibrary.Delay` _returnvalue)
    (set `self.timerRunning` false)))

(event `Fire_Projectile`
  (bind _dispersion (`self.dispersion`))
  (bind _ammo (`self.Ammo`))
  (bind _ammototal (`self.AmmoTotal`))
  (bind _ammomax (`self.AmmoMax`))
  (bind _bulletpershot (`self.bulletPerShot`))
  (bind (_returnvalue_location _returnvalue_rotation _returnvalue_scale) (`KismetMathLibrary.BreakTransform` (`SceneComponent.K2_GetComponentToWorld` (`self.Projectile_Spawn_Point`))))
  (bind _returnvalue (- 0.0 _dispersion))
  (if (> (`self.Ammo`) 0)
    (if (<= _bulletpershot _ammo)
      (for _ (range 1 (+ _bulletpershot 1))
        (bind _returnvalue_2 (`|SpawnActorFromClass` "/Game/Blueprints/Guns/BP_Projectile.BP_Projectile_C" (`KismetMathLibrary.MakeTransform` _returnvalue_location (`KismetMathLibrary.ComposeRotators` _returnvalue_rotation (`KismetMathLibrary.MakeRotator` (`KismetMathLibrary.RandomFloatInRange` _returnvalue _dispersion) (`KismetMathLibrary.RandomFloatInRange` _returnvalue _dispersion) (`KismetMathLibrary.RandomFloatInRange` _returnvalue _dispersion))) _returnvalue_scale) "Undefined" "OverrideRootScale" null null :!label _label))
        (bind _asplayer_character (cast `/Game/Blueprints/CHARACTERS/PlayerCharacter` (`GameplayStatics.GetPlayerCharacter` 0)))
        (set `/Game/Blueprints/Guns/BP_Projectile.Damage` (* (`/Game/Blueprints/CHARACTERS/PlayerCharacter.Att_gun Mul` _asplayer_character) (`self.baseDamage`) (`/Game/Blueprints/CHARACTERS/PlayerCharacter.Att Mul` _asplayer_character)) _returnvalue_2)
        (set `self.Ammo` (- (`self.Ammo`) 1))
        (`KismetSystemLibrary.PrintString` (`KismetStringLibrary.Conv_DoubleToString` 0.0)))
      (else
        (for _ (range 1 (+ _ammo 1))
          (goto _label))))
    (else
      (`KismetSystemLibrary.Delay` 2.0)
      (if (>= _ammototal _ammomax)
        (set `self.Ammo` _ammomax)
        (set `self.AmmoTotal` (- _ammototal _ammomax))
        (else
          (set `self.Ammo` _ammototal)
          (set `self.AmmoTotal` 0))))))

(fn `NewFunction_0`
  (return))

(fn `UserConstructionScript`)