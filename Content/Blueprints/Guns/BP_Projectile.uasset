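; BP_Projectile is a gun projectile that damages zombie characters it passes through.
; Begin overlap casts the other actor to ZombieCharacter, stores it and sets a colliding flag.
; End overlap, if the flag is set, subtracts Damage directly from that zombie's ZOMBIEHEALTH, clears the flag and prints the remaining health.
; Damage lands when any overlap ends, without checking which actor left.
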(event `self.ReceiveActorEndOverlap`
  (params (OtherActor :type "Actor Object Reference"))
  (bind _zombieref (`self.ZombieRef`))
  (if (`self.IsColliding`)
    (bind _output_get (set `/Game/Blueprints/CHARACTERS/ZombieCharacter.ZOMBIEHEALTH` (- (`/Game/Blueprints/CHARACTERS/ZombieCharacter.ZOMBIEHEALTH` _zombieref) (`self.Damage`)) _zombieref))
    (set `self.IsColliding` false)
    (`KismetSystemLibrary.PrintString` (`KismetStringLibrary.Conv_DoubleToString` _output_get))))

(event `self.ReceiveActorBeginOverlap`
  (params (OtherActor :type "Actor Object Reference"))
  (bind _aszombie_character (cast `/Game/Blueprints/CHARACTERS/ZombieCharacter` OtherActor))
  (set `self.IsColliding` true)
  (set `self.ZombieRef` _aszombie_character))

(fn `UserConstructionScript`)