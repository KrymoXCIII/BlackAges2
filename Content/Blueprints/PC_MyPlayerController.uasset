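; Player controller that creates the HUD widget and handles toggling of the build menu and skill window.
; On BeginPlay it caches the DEDEefault game mode, then creates the HeadsUpDisplay widget and adds it to the viewport.
; The menu input and a callable ToggleMenu event share one path that switches input mode and cursor based on the menu's returned visibility.
; The skill window input toggles through the game mode's HeadsUpDisplay reference rather than its own.
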(event `self.ReceiveBeginPlay`
  (bind _asdedeefault_game_mode (cast `/Game/Blueprints/DEDEefaultGameMode` (`GameplayStatics.GetGameMode`)))
  (set `self.MyGameMode` _asdedeefault_game_mode)
  (bind _returnvalue (`|CreateWidget` "/Game/UI/HeadsUpDisplay.HeadsUpDisplay_C"))
  (bind _output_get (set `self.HeadsUpDisplay` _returnvalue))
  (`UserWidget.AddToViewport` _output_get 0))

(event `InputAction|MENU`
  (params (Key :type "Key Structure"))
  (:`Pressed`
    (bind _returnvalue (`/Game/UI/HeadsUpDisplay.ToggleBuildMenu` (`self.HeadsUpDisplay`) :!label _label))
    (switch `ESlateVisibility` _returnvalue
      (:`Visible`
        (`WidgetBlueprintLibrary.SetInputMode_GameAndUIEx` self null)
        (set `self.bShowMouseCursor` true))
      (:`Hidden`
        (`WidgetBlueprintLibrary.SetInputMode_GameOnly` self)
        (set `self.bShowMouseCursor` false)))))

(event `ToggleMenu`
  (goto _label))

(event `InputAction|OPEN/CLOSE SKILL WINDOW`
  (params (Key :type "Key Structure"))
  (:`Pressed`
    (`/Game/Blueprints/SkillSystem/UI/HeadsUp_display_UI.ToggleSkillWindow` (`/Game/Blueprints/DEDEefaultGameMode.Heads Up Display` (`self.MyGameMode`)))))

(fn `UserConstructionScript`)