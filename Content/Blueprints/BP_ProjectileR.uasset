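; BP_ProjectileR is a projectile that damages zombies it passes through and plays a flesh-impact sound.
; Begin overlap stores the first ZombieCharacter it touches and sets IsColliding, which blocks new targets.
; Damage is applied on end overlap: it subtracts Damage from the stored zombie's ZOMBIEHEALTH, clears the flag and plays the sound.
; End overlap does not check that the exiting actor is the stored zombie.
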(event `self.ReceiveActorEndOverlap`
  (params (OtherActor :type "Actor Object Reference"))
  (bind _zombieref (`self.ZombieRef`))
  (if (`self.IsColliding`)
    (set `/Game/Blueprints/CHARACTERS/ZombieCharacter.ZOMBIEHEALTH` (- (`/Game/Blueprints/CHARACTERS/ZombieCharacter.ZOMBIEHEALTH` _zombieref) (`self.Damage`)) _zombieref)
    (set `self.IsColliding` false)
    (`GameplayStatics.PlaySoundAtLocation` "/Game/Sounds/M9FSF96-bullet-impact-flesh-54430.M9FSF96-bullet-impact-flesh-54430" (`self.K2_GetActorLocation` OtherActor) (struct) 1.0 1.0 0.0 null null null)))

(event `self.ReceiveActorBeginOverlap`
  (params (OtherActor :type "Actor Object Reference"))
  (if (not (`self.IsColliding`))
    (bind _aszombie_character (cast `/Game/Blueprints/CHARACTERS/ZombieCharacter` OtherActor))
    (set `self.IsColliding` true)
    (set `self.ZombieRef` _aszombie_character)))

(fn `UserConstructionScript`)