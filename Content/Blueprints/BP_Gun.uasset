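; BP_Gun is a gun actor that fires BP_Projectile automatically while firing is active, limited by its Ammo count.
; Fire_Start fires immediately and starts a looping timer on Fire_Projectile, which Fire_Stop clears.
; Each shot spawns at ProjectileSpawnPoint and decrements Ammo while any remains.
; Spread clamps RandomFloat (0–1) to ±Dispersion on each rotation axis, so offsets are never negative and skew one way.
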(event `Fire_Stop`
  (`KismetSystemLibrary.K2_ClearAndInvalidateTimerHandle` (stale `Fire_Start` _returnvalue)))

(event `Fire_Start`
  (`self.Fire_Projectile`)
  (bind _returnvalue (`KismetSystemLibrary.K2_SetTimerDelegate` (delegate `Fire_Projectile`) 0.3 true)))

(event `Fire_Projectile`
  (bind _dispersion (`self.dispersion`))
  (bind (_returnvalue_location _returnvalue_rotation _returnvalue_scale) (`KismetMathLibrary.BreakTransform` (`SceneComponent.K2_GetComponentToWorld` (`self.Projectile_Spawn_Point`))))
  (bind _returnvalue (- 0.0 _dispersion))
  (if (> (`self.Ammo`) 0)
    (`|SpawnActorFromClass` "/Game/Blueprints/BP_Projectile.BP_Projectile_C" (`KismetMathLibrary.MakeTransform` _returnvalue_location (`KismetMathLibrary.ComposeRotators` _returnvalue_rotation (`KismetMathLibrary.MakeRotator` (`KismetMathLibrary.FClamp` (`KismetMathLibrary.RandomFloat`) _returnvalue _dispersion) (`KismetMathLibrary.FClamp` (`KismetMathLibrary.RandomFloat`) _returnvalue _dispersion) (`KismetMathLibrary.FClamp` (`KismetMathLibrary.RandomFloat`) _returnvalue _dispersion))) _returnvalue_scale) "Undefined" "OverrideRootScale" null null)
    (set `self.Ammo` (- (`self.Ammo`) 1))))

(fn `UserConstructionScript`)