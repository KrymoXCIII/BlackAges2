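; Automated turret that, while activated, targets the nearest visible pawn of a configured class within sensing range and shoots projectiles at it.
; Each tick it picks a target via sphere overlap and line-of-sight checks, then rotates the top toward it at constant speed with clamped pitch.
; When cooled down and facing the target by dot product, a self-re-entering DoN fires two delayed right-then-left barrel volleys.
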(event `self.ReceiveTick`
  (params (DeltaSeconds :type "Float (single-precision)"))
  (if (`self.Activated`)
    (`self.FindBestTarget`)
    (`self.Target`
      (:`then`
        (`self.UpdateTurretRotation` DeltaSeconds)
        (`self.UpdateFire`))
      (:`else`))))

(event `Fire`
  (set `self.TimeOfLastFire` (`KismetSystemLibrary.GetGameTimeInSeconds`))
  (`|ExecutionSequence`
    (:`then_0`
      (goto _label :!via `Reset`))
    (:`then_1`
      (`/Engine/EditorBlueprintResources/StandardMacros.Do N` 2 :!label _label
        (:`Exit`
          (`|SpawnActorFromClass` "/Game/Blueprints/Turret/BP_Projectile.BP_Projectile_C" (`SceneComponent.GetSocketTransform` (`self.TurretBarrelR`) "Bullet" "RTS_World") "Undefined" "OverrideRootScale" null null)
          (`KismetSystemLibrary.Delay` 0.2)
          (`|SpawnActorFromClass` "/Game/Blueprints/Turret/BP_Projectile.BP_Projectile_C" (`SceneComponent.GetSocketTransform` (`self.TurretBarrelL`) "Bullet" "RTS_World") "Undefined" "OverrideRootScale" null null)
          (`KismetSystemLibrary.Delay` 0.2)
          (goto _label))))))

(fn `FindBestTarget`
  (locals (BestDistance :type "Float (double-precision)") (CurrentDistance :type "Float (double-precision)") (BestTarget :type "Actor Object Reference") (CurrentTarget :type "Actor Object Reference"))
  (set `local.BestDistance` (+ (`self.SensingRange`) 1.0))
  (bind _outactors (`KismetSystemLibrary.SphereOverlapActors` (`self.K2_GetActorLocation`) (`self.SensingRange`) (`|MakeArray` "ObjectTypeQuery3" :!type "EObjectTypeQuery Enum") (`self.TargetActorClass`)))
  (for _array_element _outactors
    (bind _output_get (set `local.CurrentTarget` _array_element))
    (bind _output_get_2 (set `local.CurrentDistance` (`self.GetDistanceTo` _output_get self)))
    (if (or (< _output_get_2 (`local.BestDistance`)) (not (`KismetSystemLibrary.IsValid` (`local.BestTarget`))))
      (bind _result (`/Game/Imported/MyFunctionLibrary.HasLineOfSight` (`SceneComponent.K2_GetComponentLocation` (`self.TurretTop`)) (`self.K2_GetActorLocation` (`local.CurrentTarget`)) (`|MakeArray` self (`local.CurrentTarget`) :!type "Actor Object Reference")))
      (if _result
        (set `local.BestTarget` (`local.CurrentTarget`))
        (set `local.BestDistance` (`local.CurrentDistance`)))))
  (set `self.Target` (`local.BestTarget`)))

(fn `UpdateFire`
  (if (> (- (`KismetSystemLibrary.GetGameTimeInSeconds`) (`self.TimeOfLastFire`)) (`self.RateOfFire`))
    (if (> (`KismetMathLibrary.Dot_VectorVector` (`KismetMathLibrary.GetDirectionUnitVector` (`SceneComponent.K2_GetComponentLocation` (`self.TurretTop`)) (`self.K2_GetActorLocation` (`self.Target`))) (`SceneComponent.GetForwardVector` (`self.TurretTop`))) 0.99)
      (`self.Fire`))))

(fn `UpdateTurretRotation`
  (params (DeltaSeconds :type "Float (double-precision)"))
  (locals (NewRotation :type "Rotator Structure" :default (struct)))
  (bind _output_get (set `local.NewRotation` (`KismetMathLibrary.RInterpTo_Constant` (`SceneComponent.K2_GetComponentRotation` (`self.TurretTop`)) (`KismetMathLibrary.FindLookAtRotation` (`SceneComponent.K2_GetComponentLocation` (`self.TurretTop`)) (`self.K2_GetActorLocation` (`self.Target`))) (`local.DeltaSeconds`) (`self.Interp Speed`))))
  (`SceneComponent.K2_SetWorldRotation` (`self.TurretTop`) (`KismetMathLibrary.MakeRotator` (.roll _output_get) (`KismetMathLibrary.ClampAngle` (.pitch _output_get) -45.0 75.0) (.yaw _output_get)) false false))

(fn `UserConstructionScript`)