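; Wave manager actor that runs enemy waves, each preceded by a short countdown.
; BeginPlay sorts all WaveSpawnPointBP actors into pools by spawner type (Zombie, Turret, Ground, Special).
; Each wave looks up its DataTable row by wave number and spawns the listed enemies at random points from the matching pool.
; A delay loop polls until no spawned enemy remains valid, then plays a sound, increments the wave and restarts the countdown.
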(event `self.ReceiveBeginPlay`
  ;[1 0 0.01752] Enemy Types
  (bind _outactors (`GameplayStatics.GetAllActorsOfClass` "/Game/Blueprints/ACTORS/Misc/WaveSpawnPointBP.WaveSpawnPointBP_C"))
  (bind _output_get (set `self.EnemySpawnPoints` _outactors))
  (for _array_element _output_get
    (switch `/Game/Enums/EnemyTypes_E` (`/Game/Blueprints/ACTORS/Misc/WaveSpawnPointBP.SpawnerType` _array_element)
      (:`NewEnumerator0`
        (`KismetArrayLibrary.Array_Add` (`self.ESP-Z`) _array_element))
      (:`NewEnumerator1`
        (`KismetArrayLibrary.Array_Add` (`self.ESP-T`) _array_element))
      (:`NewEnumerator2`
        (`KismetArrayLibrary.Array_Add` (`self.ESP-G`) _array_element))
      (:`NewEnumerator3`
        (`KismetArrayLibrary.Array_Add` (`self.ESP-S`) _array_element))))
  (`self.StartCountdown`))

(event `StartCountdown`
  ;[1 0.07388 0] COUNTDOWN
  (bind _returnvalue (`KismetSystemLibrary.K2_SetTimerDelegate` (delegate `Count`) 1.0 true))
  (set `self.Time` 5))

(event `Count`
  ;[1 0.07388 0] COUNTDOWN
  (`KismetSystemLibrary.PrintString` (`KismetStringLibrary.Conv_IntToString` (`self.Time`)))
  (`/Engine/EditorBlueprintResources/StandardMacros.DecrementInt` (`self.Time`)
    (:`  `
      (if (< (`self.Time`) 0)
        (`KismetSystemLibrary.K2_ClearAndInvalidateTimerHandle` (stale `StartCountdown` _returnvalue))
        (`self.BeginWave`)))))

(event `BeginWave`
  ;[1 0.5193 0] SPAWN ENEMIES FOR WAVE
  (`KismetSystemLibrary.PrintString` "STARTING WAVE !")
  (bind _returnvalue (`|GetDataTableRow` (`self.Data Table`) (`KismetStringLibrary.Conv_StringToName` (`KismetStringLibrary.Conv_IntToString` (`self.WaveNumber`))))
    (:`then`
      (for _array_element (`.EnemyInfos_3_FEB160074C29D713FBA184A42191076F` (break `/Game/Blueprints/STRUCTURES/WaveInfo` _returnvalue))
        (`self.SpawnEnemies` _array_element))
      (`self.AreEnemiesDeadLoop`))
    (:`RowNotFound`
      (`KismetSystemLibrary.PrintString` "Couldn't find row for Wave Data !"))))

(event `AreEnemiesDeadLoop`
  ;[0.3485 1 0] NEXT WAVE IF ENEMIES ARE DEAD
  (`KismetSystemLibrary.Delay` 1.0)
  (bind _aredead1 (`self.AreEnemiesDead`))
  (if _aredead1 :!label _label
    (`KismetSystemLibrary.PrintString` "WAVE FINISHED !")
    (`GameplayStatics.SpawnSound2D` "/Game/Packages/EasyBuildingSystem/Audio/Sounds/Interactions/Chopping/SFX_Tree_Chop_001.SFX_Tree_Chop_001" 1.0 1.0 0.0 null)
    (`/Engine/EditorBlueprintResources/StandardMacros.IncrementInt` (`self.WaveNumber`)
      (:`  `
        (`self.StartCountdown`)))
    (else
      (`KismetSystemLibrary.Delay` 1.0)
      (goto _label))))

(fn `AreEnemiesDead`
  (returns (areDead1 :type Boolean))
  (locals (areDead :type Boolean))
  (set `local.areDead` true)
  (for _array_element (`self.CurrentEnemies`)
    (`/Engine/EditorBlueprintResources/StandardMacros.IsValid` _array_element
      (:`Is Valid`
        (set `local.areDead` false))))
  (return (`local.areDead`)))

(fn `SpawnEnemies`
  (params (EnemyInfo :type "/Game/Blueprints/STRUCTURES/EnemyInfo/EnemyInfo Structure (by ref)"))
  (locals (CurrentSpawnPoints :type "Array of /Game/Blueprints/ACTORS/Misc/WaveSpawnPointBP Object Reference") (EnemyInfoRef :type "/Game/Blueprints/STRUCTURES/EnemyInfo/EnemyInfo Structure"))
  (bind _enemyinforef_enemyclass (break `/Game/Blueprints/STRUCTURES/EnemyInfo/EnemyInfo` (`local.EnemyInfoRef`)))
  (bind (_enemyinforef_enemyclass_2 _enemyinforef_enemynumber) (break `/Game/Blueprints/STRUCTURES/EnemyInfo/EnemyInfo` (`local.EnemyInfoRef`)))
  (bind _currentspawnpoints (`local.CurrentSpawnPoints`))
  (set `local.EnemyInfoRef` EnemyInfo)
  (set `local.CurrentSpawnPoints` (select `/Game/Enums/EnemyTypes_E` (`.EnemyType_8_BFD455F6463C7EF0A87521AAFF495D73` (break `/Game/Blueprints/STRUCTURES/EnemyInfo/EnemyInfo` EnemyInfo)) :`NewEnumerator0` (`self.ESP-Z`) :`NewEnumerator1` (`self.ESP-T`) :`NewEnumerator2` (`self.ESP-G`) :`NewEnumerator3` (`self.ESP-S`)))
  (for _ (range 1 (+ _enemyinforef_enemynumber 1))
    (bind _returnvalue (`|SpawnActorFromClass` _enemyinforef_enemyclass (`SceneComponent.K2_GetComponentToWorld` (`/Game/Blueprints/ACTORS/Misc/WaveSpawnPointBP.Billboard` (`|GetArrayItem` _currentspawnpoints (`KismetMathLibrary.RandomIntegerInRange` 0 (`KismetArrayLibrary.Array_LastIndex` _currentspawnpoints))))) "AdjustIfPossibleButAlwaysSpawn" "OverrideRootScale" null null))
    (`KismetArrayLibrary.Array_Add` (`self.CurrentEnemies`) _returnvalue)))

(fn `UserConstructionScript`)