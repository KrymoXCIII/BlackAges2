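; Melee axe actor that damages zombie characters when the player strikes.
; Hitbox overlap events track whether a zombie is in range, and Tick checks that flag against the player's striking state.
; A landed hit on a living zombie lowers its health by a base amount scaled by player attack multipliers, with sound, impact montage and blood effect.
; A Hit flag with a short delay limits repeat hits.
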(event `self.AxeHitbox.OnComponentBeginOverlap`
  (params (OverlappedComponent :type "PrimitiveComponent Object Reference") (OtherActor :type "Actor Object Reference") (OtherComp :type "PrimitiveComponent Object Reference") (OtherBodyIndex :type Integer) (bFromSweep :type Boolean) (SweepResult :type "HitResult Structure (by ref)"))
  (cast `/Game/Blueprints/CHARACTERS/ZombieCharacter` OtherActor)
  (bind _output_get (set `self.ZombieColliding` true)))

(event `self.AxeHitbox.OnComponentEndOverlap`
  (params (OverlappedComponent :type "PrimitiveComponent Object Reference") (OtherActor :type "Actor Object Reference") (OtherComp :type "PrimitiveComponent Object Reference") (OtherBodyIndex :type Integer))
  (cast `/Game/Blueprints/CHARACTERS/ZombieCharacter` OtherActor)
  (bind _output_get (set `self.ZombieColliding` false)))

(event `self.ReceiveTick`
  (params (DeltaSeconds :type "Float (single-precision)"))
  (bind _asplayer_character (cast `/Game/Blueprints/CHARACTERS/PlayerCharacter` (`GameplayStatics.GetPlayerCharacter` 0)))
  (if (`/Game/Blueprints/CHARACTERS/PlayerCharacter.isStriking` _asplayer_character)
    (if (`self.ZombieColliding`)
      (bind _aszombie_character (cast `/Game/Blueprints/CHARACTERS/ZombieCharacter` (stale `self.AxeHitbox.OnComponentBeginOverlap` OtherActor)))
      (if (not (`/Game/Blueprints/CHARACTERS/ZombieCharacter.isDead` _aszombie_character))
        (set `self.ZombieCharacterRef` _aszombie_character)
        (if (not (`self.Hit`))
          (set `self.Hit` true)
          (`KismetSystemLibrary.PrintString` "HIT" true true (struct :`R` 0.18964 :`G` 1.0 :`A` 1.0))
          (`GameplayStatics.PlaySound2D` "/Game/Sounds/mixkit-sword-blade-lashes-chainmail-armor-2776.mixkit-sword-blade-lashes-chainmail-armor-2776" 1.0 1.0 0.0 null null)
          (`KismetSystemLibrary.PrintString` "PLAYER ATTACK" true true (struct :`R` 0.006095 :`G` 1.0 :`B` 0.056186 :`A` 1.0))
          (set `/Game/Blueprints/CHARACTERS/ZombieCharacter.ZOMBIEHEALTH` (`KismetMathLibrary.FClamp` (- (`/Game/Blueprints/CHARACTERS/ZombieCharacter.ZOMBIEHEALTH` (`self.ZombieCharacterRef`)) (* (`/Game/Blueprints/CHARACTERS/PlayerCharacter.Att Mul` _asplayer_character) (`/Game/Blueprints/CHARACTERS/PlayerCharacter.Att_melee Mul` _asplayer_character) 35.0)) 0.0 (`/Game/Blueprints/CHARACTERS/ZombieCharacter.ZOMBIEHEALTH` _aszombie_character)) _aszombie_character)
          (`Character.PlayAnimMontage` _aszombie_character "/Game/ANIMS/ZOMBIE/RETARGETED/zombie_impact_Montage.zombie_impact_Montage" 1.0 "None")
          (`GameplayStatics.SpawnEmitterAtLocation` "/Game/Realistic_Starter_VFX_Pack_Vol2/Particles/Blood/P_Blood_Splat_Cone.P_Blood_Splat_Cone" (`self.K2_GetActorLocation` (stale `self.AxeHitbox.OnComponentBeginOverlap` OtherActor)) (struct :`Roll` 90.0))
          (`KismetSystemLibrary.Delay` 0.5)
          (set `self.Hit` false))))))

(fn `UserConstructionScript`)