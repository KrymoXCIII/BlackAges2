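; Door Blueprint that opens by destroying itself when a character interacts with it while holding the matching key.
; The Interact event switches on DoorNumber and checks the character's HasKey0, HasKey1 or HasKey2 flag for doors 0 to 2.
; Any other door number takes the default branch and destroys the door without a key check.
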(event `/Game/Blueprints/Interfaces/I_Interaction.Interact`
  (params (Character :type "/Game/Blueprints/CHARACTERS/PlayerCharacter Object Reference"))
  (switch `int` (`KismetMathLibrary.Conv_Int64ToInt` (`KismetMathLibrary.Conv_IntToInt64` (`self.DoorNumber`)))
    (:`Default`
      (`self.K2_DestroyActor` :!label _label))
    (:`0`
      (if (`/Game/Blueprints/CHARACTERS/PlayerCharacter.hasKey0` Character)
        (goto _label)))
    (:`1`
      (if (`/Game/Blueprints/CHARACTERS/PlayerCharacter.hasKey1` Character)
        (goto _label)))
    (:`2`
      (if (`/Game/Blueprints/CHARACTERS/PlayerCharacter.hasKey2` Character)
        (goto _label)))))

(fn `UserConstructionScript`)