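; NPC character that commutes between a work actor and a house actor over the navmesh and can show timed dialogue.
; MoveToWork starts on BeginPlay and alternates with MoveToHouse through AIMoveTo and pauses; a separate looping MoveNPC event is not called here.
; Overlapping another such NPC stops movement and sends TalkMessage via BPI_Dialogue to overlapping NPCs.
; Talk steps through Dialogue lines in a WB_dialogue widget, then removes it and resumes MoveToWork.
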(event `self.ReceiveActorBeginOverlap`
  (params (OtherActor :type "Actor Object Reference"))
  (`KismetSystemLibrary.PrintString` "Hello")
  (if (`GameplayStatics.ObjectIsA` OtherActor "BP_NPC_NavMesh_C")
    (`MovementComponent.StopMovementImmediately` (`self.CharacterMovement`))
    (for _array_element (`self.GetOverlappingActors` "BP_NPC_NavMesh_C")
      (if (`KismetSystemLibrary.DoesImplementInterface` _array_element "/Game/NavigationSystem/BPI_Dialogue.BPI_Dialogue_C")
        (message `/Game/NavigationSystem/BPI_Dialogue.Talk` _array_element)))))

(event `MoveToHouse`
  (set `self.MovingToHouse` true)
  (`|AIMoveTo` self (`self.K2_GetActorLocation` (`self.HouseLocation`)) null 100.0 true
    (:`OnSuccess`
      (`KismetSystemLibrary.Delay` 15.0)
      (set `self.MovingToHouse` false)
      (`self.MoveToWork`))))

(event `MoveToWork`
  (set `self.MovingToWork` true)
  (`|AIMoveTo` self (`self.K2_GetActorLocation` (`self.WorkLocation`)) null 100.0 true
    (:`OnSuccess`
      (`KismetSystemLibrary.Delay` 15.0)
      (set `self.MovingToWork` false)
      (`self.MoveToHouse`))))

(event `self.ReceiveBeginPlay`
  (`self.MoveToWork`))

(event `MoveNPC`
  (`|AIMoveTo` self (`self.K2_GetActorLocation` (`self.WorkLocation`)) null 100.0 true
    (:`OnSuccess`
      (`KismetSystemLibrary.Delay` 15.0)
      (`|AIMoveTo` self (`self.K2_GetActorLocation` (`self.HouseLocation`)) null 100.0 true
        (:`OnSuccess`
          (`KismetSystemLibrary.Delay` 15.0))
        (:`OnFail`
          _))
      (`self.MoveNPC`))
    (:`OnFail`
      (`self.MoveNPC`))))

(event `/Game/NavigationSystem/BPI_Dialogue.Talk`
  (`/Engine/EditorBlueprintResources/StandardMacros.IncrementInt` (`self.talkIndex`)
    (:`  `
      (if (< (`self.talkIndex`) (`KismetArrayLibrary.Array_Length` (`self.dialogue`)))
        (`self.UI`
          (:`then`
            _)
          (:`else`
            (bind _returnvalue (`|CreateWidget` "/Game/NavigationSystem/WB_dialogue.WB_dialogue_C" (`GameplayStatics.GetPlayerController` 0)))
            (bind _output_get (set `self.UI` _returnvalue))
            (`UserWidget.AddToViewport` _output_get 0)))
        (`TextBlock.SetText` (`/Game/NavigationSystem/WB_dialogue.TalkText` (`self.UI`)) (`KismetTextLibrary.Conv_StringToText` (`|GetArrayItem` (`self.dialogue`) (`self.talkIndex`))))
        (`KismetSystemLibrary.Delay` 5.0)
        (`/Game/NavigationSystem/BPI_Dialogue.Talk`)
        (else
          (`Widget.RemoveFromParent` (`self.UI`))
          (`self.MoveToWork`))))))

(fn `RandomItemFunc`
  (params (TargetArray :type "Array of /Game/NavigationSystem/BP_NPC_NavMesh Object Reference (by ref)"))
  (returns (OutItem :type "/Game/NavigationSystem/BP_NPC_NavMesh Object Reference"))
  (return (`KismetArrayLibrary.Array_Random` TargetArray)))

(fn `UserConstructionScript`)