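; LLMCharacter is a named NPC that the player can chat with through a local Llama language-model component.
; Entering its DetectionBox opens a dialog widget, shows the cursor and activates Llama; leaving hides the dialog and deactivates it.
; AddPrompt inserts text into Llama, generated tokens stream into the widget, and the name tag faces the camera each tick.
; Companion follow and zombie-combat logic remains in the graph but is disconnected.
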(event `self.SurvivorHitBox.OnComponentBeginOverlap`
  (params (OverlappedComponent :type "PrimitiveComponent Object Reference") (OtherActor :type "Actor Object Reference") (OtherComp :type "PrimitiveComponent Object Reference") (OtherBodyIndex :type Integer) (bFromSweep :type Boolean) (SweepResult :type "HitResult Structure (by ref)")))

(event `self.SurvivorHitBox.OnComponentEndOverlap`
  (params (OverlappedComponent :type "PrimitiveComponent Object Reference") (OtherActor :type "Actor Object Reference") (OtherComp :type "PrimitiveComponent Object Reference") (OtherBodyIndex :type Integer)))

(event `self.ReceiveTick`
  (params (DeltaSeconds :type "Float (single-precision)"))
  (`SceneComponent.K2_SetWorldRotation` (`self.NameTagWidget`) (`KismetMathLibrary.FindLookAtRotation` (`SceneComponent.K2_GetComponentLocation` (`self.NameTagWidget`)) (`self.K2_GetActorLocation` (`GameplayStatics.GetPlayerCameraManager` 0))) false false))

(event `self.ReceiveBeginPlay`
  (bind _asplayer_character (cast `/Game/Blueprints/CHARACTERS/PlayerCharacter` (`GameplayStatics.GetPlayerCharacter` 0)))
  (set `self.CharacterRef` _asplayer_character)
  (bind _aswdg_name_tag (cast `/Game/LLM/Blueprints/WDG_NameTag` (`WidgetComponent.GetWidget` (`self.NameTagWidget`))))
  (`/Game/LLM/Blueprints/WDG_NameTag.SetPlayerName` _aswdg_name_tag (`KismetTextLibrary.Conv_StringToText` (`self.Name`))))

(event `FollowPlayer`)

(event `Attack Zombie`)

(event `self.DetectionBox.OnComponentBeginOverlap`
  (params (OverlappedComponent :type "PrimitiveComponent Object Reference") (OtherActor :type "Actor Object Reference") (OtherComp :type "PrimitiveComponent Object Reference") (OtherBodyIndex :type Integer) (bFromSweep :type Boolean) (SweepResult :type "HitResult Structure (by ref)"))
  ;[0.501 1 0.2015] Test Start Talking
  (`KismetSystemLibrary.PrintString` "Begin Overlap")
  (cast `/Game/Blueprints/CHARACTERS/PlayerCharacter` OtherActor)
  (`self.StartTalking`))

(event `self.DetectionBox.OnComponentEndOverlap`
  (params (OverlappedComponent :type "PrimitiveComponent Object Reference") (OtherActor :type "Actor Object Reference") (OtherComp :type "PrimitiveComponent Object Reference") (OtherBodyIndex :type Integer))
  ;[0.5373 1 0.1143] Stop Talking
  (`KismetSystemLibrary.PrintString` "End Overlap")
  (cast `/Game/Blueprints/CHARACTERS/PlayerCharacter` OtherActor)
  (`self.StopTalking`))

(event `StartLLM`
  (`KismetSystemLibrary.PrintString` "StartLLM")
  (`WidgetBlueprintLibrary.SetInputMode_GameAndUIEx` (`GameplayStatics.GetPlayerController` 0) null)
  (set `PlayerController.bShowMouseCursor` true (`GameplayStatics.GetPlayerController` 0))
  (`ActorComponent.Activate` (`self.Llama`) false))

(event `StopLLM`
  (`KismetSystemLibrary.PrintString` "StopLLM")
  (set `PlayerController.bShowMouseCursor` false (`GameplayStatics.GetPlayerController` 0))
  (`ActorComponent.Deactivate` (`self.Llama`)))

(event `self.Llama.OnNewTokenGenerated`
  (params (NewToken :type String))
  (`/Game/Blueprints/Imported/UI/UserInterface.AddToken` (`self.UI Widget`) NewToken))

(fn `Add Prompt`
  (params (Prompt :type String))
  (`LlamaComponent.InsertPrompt` (`self.Llama`) Prompt))

(fn `StartTalking`
  (`KismetSystemLibrary.PrintString` "Start Talking")
  (bind _returnvalue (`|CreateWidget` "/Game/Blueprints/Imported/UI/UserInterface.UserInterface_C" (`GameplayStatics.GetPlayerController` 0)))
  (bind _output_get (set `self.UI Widget` _returnvalue))
  (`UserWidget.AddToViewport` _output_get 0)
  (`/Game/Blueprints/Imported/UI/UserInterface.AddDialog` _output_get)
  (`self.StartLLM`))

(fn `StopTalking`
  (`KismetSystemLibrary.PrintString` "Stop Talking")
  (`/Game/Blueprints/Imported/UI/UserInterface.HideDialog` (`self.UI Widget`))
  (`self.StopLLM`))

(fn `UserConstructionScript`)