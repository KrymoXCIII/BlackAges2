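; First-person-style player character with movement, look, jump, a pause menu and basic life and experience stats.
; BeginPlay initializes life, adds the HUD widget and starts a looping timer by function name, presumably for life decay.
; Crouch uses a timeline to lerp capsule half height, reversing on release.
; AddEXP handles level-ups with a growing threshold and sound; debug keys grant EXP and fire a line trace.
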(event `self.ReceiveBeginPlay`
  ;[1 1 1] CREATION DES DONNEES LORS DE LA CREATION DU PERSONNAGE
  (`|ExecutionSequence`
    (:`then_0`
      (set `self.CapsuleHalfHeight` (`CapsuleComponent.CapsuleHalfHeight` (`self.CapsuleComponent`))))
    (:`then_1`
      (`self.Def init stat perso`))
    (:`then_2`
      (`self.Def Base stat Actually`))
    (:`then_3`
      (`KismetSystemLibrary.K2_SetTimer` self (`self.decrement_life_name`) 5.0 true))
    (:`then_4`
      (bind _returnvalue (`|CreateWidget` "/Game/UI/UserInterface.UserInterface_C"))
      (`UserWidget.AddToViewport` _returnvalue 0))))

(event `InputAxis|Fw/Bw`
  (params (AxisValue :type "Float (single-precision)"))
  ;[0.4479 0.4357 0.4115] DEPLACEMENTS
  (`self.AddMovementInput` (`KismetMathLibrary.GetForwardVector` (`KismetMathLibrary.MakeRotator` 0.0 (.pitch (`self.GetControlRotation`)) (.yaw (`self.GetControlRotation`)))) AxisValue))

(event `InputAxis|R/L`
  (params (AxisValue :type "Float (single-precision)"))
  ;[0.4479 0.4357 0.4115] DEPLACEMENTS
  (`self.AddMovementInput` (`KismetMathLibrary.GetRightVector` (`KismetMathLibrary.MakeRotator` 0.0 (.pitch (`self.GetControlRotation`)) (.yaw (`self.GetControlRotation`)))) AxisValue))

(event `InputAxis|LU/LD`
  (params (AxisValue :type "Float (single-precision)"))
  ;[0.1117 1 0.4183] ROTATIONS
  (`self.AddControllerPitchInput` (`KismetMathLibrary.FClamp` AxisValue -5.0 5.0)))

(event `InputAxis|LR/LL`
  (params (AxisValue :type "Float (single-precision)"))
  ;[0.1117 1 0.4183] ROTATIONS
  (`self.AddControllerYawInput` (`KismetMathLibrary.FClamp` AxisValue -5.0 5.0)))

(event `InputAction|JUMP`
  (params (Key :type "Key Structure"))
  ;[1 1 1] SAUT ET S'ACCROUPIR
  (:`Pressed`
    (`self.Jump`)))

(event `InputAction|CROUCH`
  (params (Key :type "Key Structure"))
  ;[1 1 1] SAUT ET S'ACCROUPIR
  (:`Pressed`
    (`self.StartCrouch`))
  (:`Released`
    (`self.StopCrouch`)))

(event `InputAction|PAUSE GAME` :paused true
  (params (Key :type "Key Structure"))
  (bind _returnvalue (`GameplayStatics.GetPlayerController` 0))
  (bind _pause_menu_ref (`self.Pause Menu REF`))
  ;[1 1 1] Pause
  (:`Pressed`
    (`/Engine/EditorBlueprintResources/StandardMacros.IsValid` (`self.Pause Menu REF`)
      (:`Is Valid`
        _)
      (:`Is Not Valid`
        (bind _returnvalue_2 (`|CreateWidget` "/Game/UI/Import/PausedMenuWidget.PausedMenuWidget_C"))
        (set `self.Pause Menu REF` _returnvalue_2)))
    (if (`GameplayStatics.IsGamePaused`)
      (`Widget.RemoveFromParent` _pause_menu_ref)
      (`GameplayStatics.SetGamePaused` false)
      (set `PlayerController.bShowMouseCursor` false _returnvalue)
      (`WidgetBlueprintLibrary.SetInputMode_GameOnly` _returnvalue)
      (else
        (`UserWidget.AddToViewport` _pause_menu_ref 0)
        (`GameplayStatics.SetGamePaused` true)
        (set `PlayerController.bShowMouseCursor` true _returnvalue)
        (`WidgetBlueprintLibrary.SetInputMode_GameAndUIEx` _returnvalue _pause_menu_ref "LockInFullscreen" false)))))

(event `StartCrouch`
  (set `self.IsCrouched` true)
  (bind (_direction _lerpvalue) (`Timeline|CrouchSmooth` :!label _label)
    (:`Update`
      (`CapsuleComponent.SetCapsuleHalfHeight` (`self.CapsuleComponent`) (`KismetMathLibrary.Lerp` (`self.CapsuleHalfHeight`) (`CharacterMovementComponent.CrouchedHalfHeight` (`self.CharacterMovement`)) _lerpvalue) true))))

(event `StopCrouch`
  (set `self.IsCrouched` false)
  (goto _label :!via `Reverse`))

(event `Key|A`
  (params (Key :type "Key Structure"))
  (:`Pressed`
    (`KismetSystemLibrary.LineTraceSingle` :`Start` (`self.K2_GetActorLocation`) :`End` (* (`KismetMathLibrary.GetForwardVector` (`self.GetControlRotation`)) 150.0) :`TraceChannel` "TraceTypeQuery1" :`DrawDebugType` "Persistent")
    (`KismetSystemLibrary.PrintString` "Hello")))

(event `Key|D`
  (params (Key :type "Key Structure"))
  (:`Pressed`
    (`self.Add EXP` 5)))

(fn `Add EXP`
  (params (EXP :type Integer))
  (returns (Level :type Integer))
  (bind _output_get (set `self.EXP` (+ EXP (`self.EXP`))))
  (if (>= _output_get (`self.EXP Needed`))
    (`/Engine/EditorBlueprintResources/StandardMacros.IncrementInt` (`self.Level`)
      (:`  `
        (set `self.EXP` (- (`self.EXP`) (`self.EXP Needed`)))
        (set `self.EXP Needed` (`KismetMathLibrary.Clamp` (`KismetMathLibrary.FTrunc` (* (`self.EXP Needed`) 1.2)) 0 1000))
        (`GameplayStatics.PlaySound2D` "/Game/Sounds/LevelUp.LevelUp" 1.0 1.0 0.0 null null)
        (return (`self.Level`))))))

(fn `decrease life`
  (bind _returnvalue (`KismetMathLibrary.FClamp` (- (`self.Life_Actually`) (`self.Life_decrement`)) 0.0 (`self.Life_base`)))
  (if (not (<= _returnvalue 0.0))
    (set `self.Life_Actually` _returnvalue)))

(fn `Def Base stat Actually`
  (set `self.Life_Actually` (`self.Life_base`)))

(fn `Def init stat perso`
  (set `self.Life_base` 100.0))

(fn `UserConstructionScript`)